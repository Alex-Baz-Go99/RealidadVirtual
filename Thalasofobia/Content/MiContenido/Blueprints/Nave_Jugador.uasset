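; Player ship pawn that flies along its own axes, with mouse look on the camera.
; Turn and LookUp accumulate clamped yaw and pitch offsets, applied as the camera's relative rotation.
; Rotate axes add into a separate unclamped yaw that sets the collision component's world rotation.
; Move axes feed AddMovementInput along actor forward, right and up vectors; opposing up/down and rotate handlers share identical logic, so direction depends on axis sign.
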(event Input|AxisEvents|InputAxisMoveUp
  (params (AxisValue :type Float%20%28single-precision%29))
  (Pawn|Input|AddMovementInput (Transformation|GetActorUpVector) AxisValue false))

(event Input|AxisEvents|InputAxisMoveForward
  (params (AxisValue :type Float%20%28single-precision%29))
  (Pawn|Input|AddMovementInput (Transformation|GetActorForwardVector) AxisValue false))

(event Input|AxisEvents|InputAxisMoveRight
  (params (AxisValue :type Float%20%28single-precision%29))
  (Pawn|Input|AddMovementInput (Transformation|GetActorRightVector) AxisValue false))

(event Input|AxisEvents|InputAxisRotateLeft
  (params (AxisValue :type Float%20%28single-precision%29))
  (bind _output_get (Variables|Default|SetRot_Delta_Turn (+ AxisValue (Variables|Default|GetRot_Delta_Turn))))
  (Transformation|SetWorldRotation (Variables|Default|GetCollisionComponent) (Math|Rotator|MakeRotator 0.0 0.0 _output_get) false false))

(event Input|AxisEvents|InputAxisRotateRight
  (params (AxisValue :type Float%20%28single-precision%29))
  (bind _output_get (Variables|Default|SetRot_Delta_Turn (+ AxisValue (Variables|Default|GetRot_Delta_Turn))))
  (Transformation|SetWorldRotation (Variables|Default|GetCollisionComponent) (Math|Rotator|MakeRotator 0.0 0.0 _output_get) false false))

(event Input|AxisEvents|InputAxisLookUp
  (params (AxisValue :type Float%20%28single-precision%29))
  ;[1 1 1] Mirar con mouse
  (bind _output_get (Variables|Default|SetRot_Delta_Y (Math|Float|Clamp(Float) (+ AxisValue (Variables|Default|GetRot_Delta_Y)) -5e+01 7e+01)))
  (Transformation|SetRelativeRotation (Variables|Default|GetCamera) (Math|Rotator|MakeRotator 0.0 _output_get (stale Input|AxisEvents|InputAxisTurn _output_get)) false false))

(event Input|AxisEvents|InputAxisMoveDown
  (params (AxisValue :type Float%20%28single-precision%29))
  (Pawn|Input|AddMovementInput (Transformation|GetActorUpVector) AxisValue false))

(event Input|AxisEvents|InputAxisTurn
  (params (AxisValue :type Float%20%28single-precision%29))
  ;[1 1 1] Mirar con mouse
  (bind _output_get (Variables|Default|SetRot_Delta (Math|Float|Clamp(Float) (+ AxisValue (Variables|Default|GetRot_Delta)) -1e+02 1e+02)))
  (Transformation|SetRelativeRotation (Variables|Default|GetCamera) (Math|Rotator|MakeRotator 0.0 (stale Input|AxisEvents|InputAxisLookUp _output_get) _output_get) false false))

(fn ConstructionScript)
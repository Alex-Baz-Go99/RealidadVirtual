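; Ship pawn (Nave) Blueprint that handles look input for its camera, with no movement logic in its graphs.
; Turn and LookUp axes accumulate into clamped yaw and pitch offsets, applied as the Camera's relative rotation for limited free look.
; TurnRate and LookUpRate instead add controller yaw and pitch, scaled by base rates and frame delta time.
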(event EventBeginPlay)

(event Collision|EventActorBeginOverlap
  (params (OtherActor :type Actor%20Object%20Reference)))

(event EventTick
  (params (DeltaSeconds :type Float%20%28single-precision%29)))

(event Input|AxisEvents|InputAxisLookUp
  (params (AxisValue :type Float%20%28single-precision%29))
  ;[1 1 1] Mirar con mouse
  (bind _output_get (Variables|Default|SetRot_Delta_Y (Math|Float|Clamp(Float) (+ AxisValue (Variables|Default|GetRot_Delta_Y)) -5e+01 7e+01)))
  (Transformation|SetRelativeRotation (Variables|Default|GetCamera) (Math|Rotator|MakeRotator 0.0 _output_get (stale Input|AxisEvents|InputAxisTurn _output_get)) false false))

(event Input|AxisEvents|InputAxisTurnRate
  (params (AxisValue :type Float%20%28single-precision%29))
  (Pawn|Input|AddControllerYawInput (* AxisValue (Variables|Default|GetBase_Turn_Rate) (Utilities|Time|GetWorldDeltaSeconds))))

(event Input|AxisEvents|InputAxisTurn
  (params (AxisValue :type Float%20%28single-precision%29))
  ;[1 1 1] Mirar con mouse
  (bind _output_get (Variables|Default|SetRot_Delta (Math|Float|Clamp(Float) (+ AxisValue (Variables|Default|GetRot_Delta)) -1e+02 1e+02)))
  (Transformation|SetRelativeRotation (Variables|Default|GetCamera) (Math|Rotator|MakeRotator 0.0 (stale Input|AxisEvents|InputAxisLookUp _output_get) _output_get) false false))

(event Input|AxisEvents|InputAxisLookUpRate
  (params (AxisValue :type Float%20%28single-precision%29))
  (Pawn|Input|AddControllerPitchInput (* AxisValue (Variables|Default|GetBase_Look_Up_Rate) (Utilities|Time|GetWorldDeltaSeconds))))

(fn ConstructionScript)